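; Sword actor with a Box hit volume that calls ApplyDamage using SwordDamage.
; SwordActive and SwordDeactive events switch the Box collision on and off.
; Overlaps with actors other than the player pawn pass a DoOnce that resets after a short delay, but ApplyDamage has no target wired.
; Tick polls two gamepad face buttons to switch between low and high damage, printing the value.
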(event `self.ReceiveTick`
  (params (DeltaSeconds :type "Float (single-precision)"))
  (bind _returnvalue (`GameplayStatics.GetPlayerController` 0))
  (if (`PlayerController.WasInputKeyJustPressed` _returnvalue "Gamepad_FaceButton_Left")
    (bind _output_get (set `self.Sword Damage` 1.0))
    (`KismetSystemLibrary.PrintString` (`KismetStringLibrary.Conv_DoubleToString` _output_get))
    (elif (`PlayerController.WasInputKeyJustPressed` _returnvalue "Gamepad_FaceButton_Top")
      (bind _output_get_2 (set `self.Sword Damage` 10.0))
      (`KismetSystemLibrary.PrintString` (`KismetStringLibrary.Conv_DoubleToString` _output_get_2)))))

(event `self.Box.OnComponentBeginOverlap`
  (params (OverlappedComponent :type "PrimitiveComponent Object Reference") (OtherActor :type "Actor Object Reference") (OtherComp :type "PrimitiveComponent Object Reference") (OtherBodyIndex :type Integer) (bFromSweep :type Boolean) (SweepResult :type "HitResult Structure (by ref)"))
  (if (!= OtherActor (`GameplayStatics.GetPlayerPawn` 0))
    (`/Engine/EditorBlueprintResources/StandardMacros.DoOnce` false :!label _label
      (:`Completed`
        (`GameplayStatics.ApplyDamage` null (`self.Sword Damage`))
        (`KismetSystemLibrary.Delay` 0.1)
        (goto _label :!via `Reset`)))))

(event `SwordActive`
  (`PrimitiveComponent.SetCollisionProfileName` (`self.Box`) "OverlapAll" true))

(event `SwordDeactive`
  (`PrimitiveComponent.SetCollisionEnabled` (`self.Box`) "NoCollision"))

(fn `UserConstructionScript`)